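; Player character Blueprint for the Advanced Locomotion System (ALS) that tailors animations and held props to the current overlay state.
; Input events forward movement, camera, stance, jump, aim and combat actions to handler functions.
; Switches on OverlayState pick get-up, landing-roll and low-mantle assets by hand usage and attach the matching weapon or prop.
; The bow's AnimBP draw value follows the Enable_SpineRotation curve.
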(event `self.UpdateHeldObjectAnimations`
  ;[0.6298 1 0.5647] BP Implementable Events
  (`self.OnUpdateHeldObjectAnimations`))

(event `self.UpdateHeldObject`
  ;[0.6298 1 0.5647] BP Implementable Events
  (`self.OnUpdateHeldObject`))

(event `InputAxis|MoveForward/Backwards`
  (params (AxisValue :type "Float (single-precision)"))
  (`self.PlayerForwardMovementInput` AxisValue))

(event `InputAxis|MoveRight/Left`
  (params (AxisValue :type "Float (single-precision)"))
  (`self.PlayerRightMovementInput` AxisValue))

(event `InputAxis|LookUp/Down`
  (params (AxisValue :type "Float (single-precision)"))
  (`self.PlayerCameraUpInput` AxisValue))

(event `InputAxis|LookLeft/Right`
  (params (AxisValue :type "Float (single-precision)"))
  (`self.PlayerCameraRightInput` AxisValue))

(event `InputAction|SprintAction`
  (params (Key :type "Key Structure"))
  (:`Pressed`
    (`self.SprintPressedAction`))
  (:`Released`
    (`self.SprintReleasedAction`)))

(event `InputAction|WalkAction`
  (params (Key :type "Key Structure"))
  (:`Pressed`
    (`self.WalkPressedAction`)))

(event `InputAction|JumpAction`
  (params (Key :type "Key Structure"))
  (:`Pressed`
    (`self.JumpPressedAction`))
  (:`Released`
    (`self.JumpReleasedAction`)))

(event `InputAction|AimAction`
  (params (Key :type "Key Structure"))
  (:`Pressed`
    (`self.AimPressedAction`))
  (:`Released`
    (`self.AimReleasedAction`)))

(event `InputAction|FireAction`
  (params (Key :type "Key Structure"))
  (:`Pressed`
    (`self.CombatModePressed`))
  (:`Released`
    (`self.CombatModeReleased`)))

(event `InputAction|StanceAction`
  (params (Key :type "Key Structure"))
  (:`Pressed`
    (`self.StancePressedAction`)))

(fn `GetGetUpAnimation`
  (params (bRagdollFaceUpState :type Boolean))
  (returns (ReturnValue :type "AnimMontage Object Reference"))
  (if bRagdollFaceUpState
    (switch `EALSOverlayState` (`self.OverlayState`)
      (:`Default`
        _)
      (:`Masculine`
        _)
      (:`Feminine`
        _)
      (:`Injured`
        (return (`self.GetUpBack_LH`)))
      (:`HandsTied`
        (return (`self.GetUpBack_2H`)))
      (:`Rifle`
        (return (`self.GetUpBack_RH`)))
      (:`PistolOneHanded`
        (return (`self.GetUpBack_RH`)))
      (:`PistolTwoHanded`
        (return (`self.GetUpBack_RH`)))
      (:`Bow`
        (return (`self.GetUpBack_LH`)))
      (:`Torch`
        (return (`self.GetUpBack_LH`)))
      (:`Binoculars`
        (return (`self.GetUpBack_RH`)))
      (:`Box`
        (return (`self.GetUpBack_2H`)))
      (:`Barrel`
        (return (`self.GetUpBack_LH`))))
    (return (`self.GetUpBack_Default`))
    (else
      (switch `EALSOverlayState` (`self.OverlayState`)
        (:`Default`
          _)
        (:`Masculine`
          _)
        (:`Feminine`
          _)
        (:`Injured`
          (return (`self.GetUpFront_LH`)))
        (:`HandsTied`
          (return (`self.GetUpFront_2H`)))
        (:`Rifle`
          (return (`self.GetUpFront_RH`)))
        (:`PistolOneHanded`
          (return (`self.GetUpFront_RH`)))
        (:`PistolTwoHanded`
          (return (`self.GetUpFront_RH`)))
        (:`Bow`
          (return (`self.GetUpFront_LH`)))
        (:`Torch`
          (return (`self.GetUpFront_LH`)))
        (:`Binoculars`
          (return (`self.GetUpFront_RH`)))
        (:`Box`
          (return (`self.GetUpFront_2H`)))
        (:`Barrel`
          (return (`self.GetUpFront_LH`))))
      (return (`self.GetUpFront_Default`)))))

(fn `GetMantleAsset`
  (params (MantleType :type "EALSMantleType Enum" :default "HighMantle"))
  (returns (ReturnValue :type "ALSMantleAsset Structure"))
  (switch `EALSMantleType` MantleType
    (:`HighMantle`
      _)
    (:`LowMantle`
      (switch `EALSOverlayState` (`self.OverlayState`)
        (:`Default`
          _)
        (:`Masculine`
          _)
        (:`Feminine`
          _)
        (:`Injured`
          (return (`self.Mantle_1m_LH`)))
        (:`HandsTied`
          (return (`self.Mantle_1m_2H`)))
        (:`Rifle`
          (return (`self.Mantle_1m_RH`)))
        (:`PistolOneHanded`
          (return (`self.Mantle_1m_RH`)))
        (:`PistolTwoHanded`
          (return (`self.Mantle_1m_RH`)))
        (:`Bow`
          (return (`self.Mantle_1m_LH`)))
        (:`Torch`
          (return (`self.Mantle_1m_LH`)))
        (:`Binoculars`
          (return (`self.Mantle_1m_RH`)))
        (:`Box`
          (return (`self.Mantle_1m_Box`)))
        (:`Barrel`
          (return (`self.Mantle_1m_LH`))))
      (return (`self.Mantle_1m_Default`)))
    (:`FallingCatch`
      _))
  (return (`self.Mantle_2m_Default`)))

(fn `GetRollAnimation`
  (returns (ReturnValue :type "AnimMontage Object Reference"))
  (switch `EALSOverlayState` (`self.OverlayState`)
    (:`Default`
      _)
    (:`Masculine`
      _)
    (:`Feminine`
      _)
    (:`Injured`
      (return (`self.LandRoll_LH`)))
    (:`HandsTied`
      (return (`self.LandRoll_2H`)))
    (:`Rifle`
      (return (`self.LandRoll_2H`)))
    (:`PistolOneHanded`
      (return (`self.LandRoll_RH`)))
    (:`PistolTwoHanded`
      (return (`self.LandRoll_RH`)))
    (:`Bow`
      (return (`self.LandRoll_LH`)))
    (:`Torch`
      (return (`self.LandRoll_LH`)))
    (:`Binoculars`
      (return (`self.LandRoll_2H`)))
    (:`Box`
      (return (`self.LandRoll_2H`)))
    (:`Barrel`
      (return (`self.LandRoll_LH`))))
  (return (`self.LandRoll_Default`)))

(fn `OnUpdateHeldObject`
  (switch `EALSOverlayState` (`self.OverlayState`)
    (:`Default`
      (`self.ClearHeldObject` :!label _label))
    (:`Masculine`
      (goto _label))
    (:`Feminine`
      (goto _label))
    (:`Injured`
      (goto _label))
    (:`HandsTied`
      (goto _label))
    (:`Rifle`
      (`self.AttachToHand` null "/ALS/Props/Meshes/M4A1.M4A1"))
    (:`PistolOneHanded`
      (`self.AttachToHand` null "/ALS/Props/Meshes/M9.M9"))
    (:`PistolTwoHanded`
      (`self.AttachToHand` null "/ALS/Props/Meshes/M9.M9"))
    (:`Bow`
      (`self.AttachToHand` null "/ALS/Props/Meshes/Bow.Bow" null true))
    (:`Torch`
      (`self.AttachToHand` "/ALS/Props/Meshes/Torch.Torch" null null true))
    (:`Binoculars`
      (`self.AttachToHand` "/ALS/Props/Meshes/Binoculars.Binoculars"))
    (:`Box`
      (`self.AttachToHand` "/ALS/Props/Meshes/Box.Box"))
    (:`Barrel`
      (`self.AttachToHand` "/ALS/Props/Meshes/Barrel.Barrel" null null true))))

(fn `OnUpdateHeldObjectAnimations`
  (switch `EALSOverlayState` (`self.OverlayState`)
    (:`Bow`
      (bind _asbow_anim_bp (cast `/ALS/Props/Meshes/Bow_AnimBP` (`SkeletalMeshComponent.GetAnimInstance` (`self.SkeletalMesh`))))
      (set `/ALS/Props/Meshes/Bow_AnimBP.Draw` (`self.GetAnimCurveValue` "Enable_SpineRotation") _asbow_anim_bp))))

(fn `UserConstructionScript`
  (`parent.UserConstructionScript`))